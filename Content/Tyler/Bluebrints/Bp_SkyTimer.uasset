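; Day/night cycle actor that rotates the level's first directional light and keeps a countdown for the current phase.
; TimeSwap alternates between night and day timelines that drive light pitch, adding an audio component per phase and flipping IsNight when each finishes.
; Day hands over immediately, while night waits through an extra delay before looping.
; SkyTimer resets Time per phase, and a Delay on Tick decrements it each second to update Percenttime.
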(event Custom|TimeSwap
  (bind _directionlight (Variables|Default|GetDirectionLight))
  (bind _directionlight_2 (Variables|Default|GetDirectionLight))
  ;[1 1 1] Time swap function
  (Variables|Default|SetNightTimer false)
  (if (Variables|Default|GetIsNight)
    (CallFunction|SkyTimer)
    (bind _returnvalue (AddComponent|AddAudioComponent false))
    (Variables|Default|SetNewVar _returnvalue)
    (bind _nightcycle (Timeline|NightCycle PlayFromStart)
      (:Update
        (Transformation|SetActorRelativeRotation _directionlight_2 (Math|Rotator|MakeRotator 0.0 _nightcycle 0.0)))
      (:Finished
        (Variables|Default|SetIsNight false)
        (Class|LightComponent|SetTemperature (Variables|/Script/Engine.Light|GetLightComponent _directionlight_2) 6.5e+03)
        (Variables|Default|SetNightTimer true)
        (Variables|Default|SetTime 1.2e+02)
        (Utilities|FlowControl|Delay 1.2e+02)
        (Audio|Components|Audio|Stop (Variables|Default|GetNewVar_0))
        (CallFunction|TimeSwap :!label _label)))
    (else
      (CallFunction|SkyTimer)
      (bind _returnvalue_2 (AddComponent|AddAudioComponent false))
      (Variables|Default|SetNewVar_0 _returnvalue_2)
      (bind _daycycle (Timeline|Daycycle PlayFromStart)
        (:Update
          (Transformation|SetActorRelativeRotation _directionlight (Math|Rotator|MakeRotator 0.0 _daycycle 0.0)))
        (:Finished
          (Variables|Default|SetIsNight true)
          (Class|LightComponent|SetTemperature (Variables|/Script/Engine.Light|GetLightComponent _directionlight) 6.5e+03)
          (Audio|Components|Audio|Stop (Variables|Default|GetNewVar))
          (goto _label))))))

(event Custom|SkyTimer
  ;[1 1 1] Sets how long timer will last
  (if (Variables|Default|GetIsNight)
    (Variables|Default|SetTime 6e+01)
    (else
      (Variables|Default|SetTime 1.2e+02))))

(event EventBeginPlay
  ;[1 1 1] Ref to light and sky dome, calls timer function
  (bind _outactors (Actor|GetAllActorsOfClass "/Script/Engine.DirectionalLight"))
  (Variables|Default|SetDirectionLight (Utilities|Array|Get(acopy) _outactors))
  (CallFunction|TimeSwap)
  (Utilities|FlowControl|Delay 6e+01)
  (Variables|Default|SetMaxTime 1.2e+02))

(event EventTick
  (params (DeltaSeconds :type Float%20%28single-precision%29))
  ;[1 1 1] Update time every second
  (Utilities|FlowControl|Delay 1.0)
  (Math|Float|DecrementFloat (Variables|Default|GetTime)
    (:%20%20
      (Variables|Default|SetPercenttime (/ (Variables|Default|GetTime) (Variables|Default|GetMaxTime))))))

(fn ConstructionScript)