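; Basic night-time enemy that chases whichever of the two Synty third-person player characters is nearer and destroys itself once the sky timer leaves night.
; BeginPlay runs a repeating AI MoveTo loop, picking the target by comparing 2D distances.
; On arrival it deals damage on a one-second cooldown, unless the player is well above it.
; UpdateHealth applies player damage, briefly halting movement as a stagger, or credits the kill and destroys the enemy at zero health.
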(event Custom|AddStagger
  (bind _charactermovement (Variables|Character|GetCharacterMovement))
  ;[1 1 1] Stagger enemy
  (Variables|/Script/Engine.CharacterMovementComponent|SetMaxWalkSpeed _charactermovement 0.0)
  (Utilities|FlowControl|Delay 0.5)
  (Variables|/Script/Engine.CharacterMovementComponent|SetMaxWalkSpeed _charactermovement 2e+02))

(event Custom|UpdateHealth
  (params (Playerdamage :type Float%20%28double-precision%29) (Player :type BP%20Third%20Person%20Character%20Synty%20Object%20Reference))
  ;[1 1 1] Update enemy health
  (Variables|Default|SetCurrentHealth (- (Variables|Default|GetCurrentHealth) Playerdamage))
  (if (> (Variables|Default|GetCurrentHealth) 0.0)
    (CallFunction|AddStagger)
    (Development|PrintString (Utilities|String|ToString(Float) (Variables|Default|GetCurrentHealth)))
    (else
      (Default|AddKill Player)
      (Actor|DestroyActor))))

(event EventBeginPlay
  (bind _self self)
  (bind _capsulecomponent (Variables|Collision|GetCapsuleComponent _self))
  (bind _returnvalue (Transformation|GetWorldLocation _capsulecomponent))
  ;[1 1 1] Enemy Move
  ;;[1 1 1] Ref to sky timer
  (bind _outactors (Actor|GetAllActorsOfClass "/Game/Tyler/Bluebrints/Bp_SkyTimer.Bp_SkyTimer_C"))
  (Variables|Default|SetSkyTimerRef (Utilities|Array|Get(acopy) _outactors))
  (bind _outactors_2 (Actor|GetAllActorsOfClass "/Game/ThirdPerson/Blueprints/BP_ThirdPersonCharacterSynty.BP_ThirdPersonCharacterSynty_C"))
  (AI|AIMoveTo self "0, 0, 0" (select (> (Math|Vector|Distance(Vector) (Math|Vector|MakeVector (.x _returnvalue) (.y _returnvalue) 0.0) (Math|Vector|MakeVector (.x (Transformation|GetWorldLocation (Variables|/Script/Engine.Character|GetCapsuleComponent (Utilities|Array|Get(acopy) _outactors_2)))) (.y (Transformation|GetWorldLocation (Variables|/Script/Engine.Character|GetCapsuleComponent (Utilities|Array|Get(acopy) _outactors_2)))) 0.0)) (Math|Vector|Distance(Vector) (Math|Vector|MakeVector (.x _returnvalue) (.y _returnvalue) 0.0) (Math|Vector|MakeVector (.x (Transformation|GetWorldLocation (Variables|/Script/Engine.Character|GetCapsuleComponent (Utilities|Array|Get(acopy) _outactors_2 1)))) (.y (Transformation|GetWorldLocation (Variables|/Script/Engine.Character|GetCapsuleComponent (Utilities|Array|Get(acopy) _outactors_2 1)))) 0.0))) (Utilities|Array|Get(acopy) _outactors_2 1) (Utilities|Array|Get(acopy) _outactors_2)) 5.0 false :!label _label
    (:then
      (Utilities|FlowControl|Delay 0.2 :!label _label_2)
      (goto _label))
    (:OnSuccess
      (if (not (> (.z (Transformation|GetWorldLocation (Variables|/Script/Engine.Actor|GetRootComponent (select (> (Math|Vector|Distance(Vector) (Math|Vector|MakeVector (.x _returnvalue) (.y _returnvalue) 0.0) (Math|Vector|MakeVector (.x (Transformation|GetWorldLocation (Variables|/Script/Engine.Character|GetCapsuleComponent (Utilities|Array|Get(acopy) _outactors_2)))) (.y (Transformation|GetWorldLocation (Variables|/Script/Engine.Character|GetCapsuleComponent (Utilities|Array|Get(acopy) _outactors_2)))) 0.0)) (Math|Vector|Distance(Vector) (Math|Vector|MakeVector (.x _returnvalue) (.y _returnvalue) 0.0) (Math|Vector|MakeVector (.x (Transformation|GetWorldLocation (Variables|/Script/Engine.Character|GetCapsuleComponent (Utilities|Array|Get(acopy) _outactors_2 1)))) (.y (Transformation|GetWorldLocation (Variables|/Script/Engine.Character|GetCapsuleComponent (Utilities|Array|Get(acopy) _outactors_2 1)))) 0.0))) (Utilities|Array|Get(acopy) _outactors_2 1) (Utilities|Array|Get(acopy) _outactors_2))))) (+ (.z (Transformation|GetWorldLocation (Variables|Collision|GetCapsuleComponent))) 2e+02))) ; Check Player hight
        (Utilities|FlowControl|DoOnce false :!label _label_3
          (:Completed
            (if (> (Math|Vector|Distance(Vector) (Math|Vector|MakeVector (.x _returnvalue) (.y _returnvalue) 0.0) (Math|Vector|MakeVector (.x (Transformation|GetWorldLocation (Variables|/Script/Engine.Character|GetCapsuleComponent (Utilities|Array|Get(acopy) _outactors_2)))) (.y (Transformation|GetWorldLocation (Variables|/Script/Engine.Character|GetCapsuleComponent (Utilities|Array|Get(acopy) _outactors_2)))) 0.0)) (Math|Vector|Distance(Vector) (Math|Vector|MakeVector (.x _returnvalue) (.y _returnvalue) 0.0) (Math|Vector|MakeVector (.x (Transformation|GetWorldLocation (Variables|/Script/Engine.Character|GetCapsuleComponent (Utilities|Array|Get(acopy) _outactors_2 1)))) (.y (Transformation|GetWorldLocation (Variables|/Script/Engine.Character|GetCapsuleComponent (Utilities|Array|Get(acopy) _outactors_2 1)))) 0.0))) ; Player 2 true, player 1 false
              ;;[1 1 1] Damage
              (Default|TakeDamage (Utilities|Array|Get(acopy) _outactors_2 1) 2e+01) ; Player 2
              (else
                (Default|TakeDamage (Utilities|Array|Get(acopy) _outactors_2) 2e+01) ; Player one
              ))
            (Utilities|FlowControl|Delay 1.0)
            (goto _label_3 Reset)))))
    (:OnFail
      (goto _label_2))))

(event EventTick
  (params (DeltaSeconds :type Float%20%28single-precision%29))
  ;[1 1 1] Check if day
  (Utilities|FlowControl|Delay 1.0)
  (if (not (Variables|/Game/Tyler/Bluebrints/Bp_SkyTimer.Bp_SkyTimer_C|GetNightTimer (Variables|Default|GetSkyTimerRef)))
    (Actor|DestroyActor)))

(fn ConstructionScript)