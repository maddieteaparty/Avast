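; Boss enemy that chases the nearer of two players, deals sweep damage on reaching them and summons attacks.
; An AI MoveTo loop re-targets by distance, with a DoOnce cooldown on the sweep.
; A self-re-triggering random event periodically fires a shark projectile or spawns basic/advanced enemies at two points.
; Hits update the health widget and briefly halt movement; death credits the player's kill, while the daytime despawn check is unconnected.
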(event Custom|SharkAttack
  (params (PlayerTarget :type Actor%20Object%20Reference))
  (bind _sharksplash (Variables|Default|GetSharkSplash))
  ;[1 1 1] Shark attack
  (Animation|StopAnimMontage "/Game/Developers/dynod/SmallAttack.SmallAttack")
  (Animation|StopAnimMontage "/Game/Developers/dynod/SwingBoss.SwingBoss")
  (Animation|PlayAnimMontage "/Game/Developers/dynod/SpawnShark.SpawnShark" 1.0 "None")
  (Utilities|FlowControl|Delay 0.5)
  (Rendering|ToggleVisibility _sharksplash false)
  (Game|SpawnActorfromClass "/Game/Tyler/Bluebrints/BP_SharkProjectile.BP_SharkProjectile_C" (Transformation|GetWorldTransform (Variables|Default|GetSharkSpawn)) "AlwaysSpawn" "MultiplyWithRoot" 0 0)
  (Utilities|FlowControl|Delay 0.5)
  (Rendering|ToggleVisibility _sharksplash false)
  (Development|PrintString "sark attack"))

(event Custom|UpdateHealth
  (params (Playerdamage :type Float%20%28double-precision%29) (Player :type BP%20Third%20Person%20Character%20Synty%20Object%20Reference))
  ;[1 1 1] Update enemy health
  (Variables|Default|SetCurrentHealth (- (Variables|Default|GetCurrentHealth) Playerdamage))
  (if (> (Variables|Default|GetCurrentHealth) 0.0)
    (CallFunction|AddStagger)
    (CallFunction|UpdateHealthWidget)
    (else
      (Default|AddKill Player)
      (Actor|DestroyActor))))

(event Custom|UpdateHealthWidget
  ;[1 1 1] Update health on the widget
  (bind _asw_enemy_health (Utilities|Casting|CastToW_EnemyHealth (UserInterface|GetUserWidgetObject (Variables|Default|GetHealthBar))))
  (Default|UpdateHealthBar _asw_enemy_health (Variables|Default|GetCurrentHealth) (Variables|Default|GetMaxHealth)))

(event Custom|SpawnMoreSkels
  (params (Player%20Target :type Actor%20Object%20Reference))
  ;[1 1 1] Spawn skels
  (Animation|StopAnimMontage "/Game/Developers/dynod/SwingBoss.SwingBoss")
  (Animation|StopAnimMontage "/Game/Developers/dynod/SmallAttack.SmallAttack")
  (Animation|PlayAnimMontage "/Game/Developers/dynod/SpawnSkeles.SpawnSkeles" 1.0 "None")
  (Utilities|FlowControl|Delay 0.5)
  (switch int (Math|Random|RandomInteger 2)
    (:Default
      (AI|SpawnAIFromClass "/Game/Tyler/Bluebrints/BP_EnemyBasic.BP_EnemyBasic_C" 0 (Transformation|GetWorldLocation (Variables|Default|GetSpawnPoint2)) "0, 0, 0" false 0 :!label _label)
      (AI|SpawnAIFromClass "/Game/Tyler/Bluebrints/BP_EnemyBasic.BP_EnemyBasic_C" 0 (Transformation|GetWorldLocation (Variables|Default|GetSpawnPoint1)) "0, 0, 0" false 0))
    (:0
      (goto _label))
    (:1
      (AI|SpawnAIFromClass (select (Math|Random|RandomBool) "/Game/Tyler/Bluebrints/BP_EnemyAdvanced.BP_EnemyAdvanced_C" "/Game/Tyler/Bluebrints/BP_EnemyBasic.BP_EnemyBasic_C") 0 (Transformation|GetWorldLocation (Variables|Default|GetSpawnPoint2)) "0, 0, 0" false 0)
      (AI|SpawnAIFromClass (select (Math|Random|RandomBool) "/Game/Tyler/Bluebrints/BP_EnemyAdvanced.BP_EnemyAdvanced_C" "/Game/Tyler/Bluebrints/BP_EnemyBasic.BP_EnemyBasic_C") 0 (Transformation|GetWorldLocation (Variables|Default|GetSpawnPoint1)) "0, 0, 0" false 0))
    (:2
      (AI|SpawnAIFromClass (Utilities|Select :Index (Math|Random|RandomInteger 3) :Option%200 "/Game/Tyler/Bluebrints/BP_EnemyBasic.BP_EnemyBasic_C" :Option%201 "/Game/Tyler/Bluebrints/BP_EnemyAdvanced.BP_EnemyAdvanced_C" :Option%202 "/Game/Tyler/Bluebrints/BP_EnemyAdvanced.BP_EnemyAdvanced_C" :Option%203 "/Game/Tyler/Bluebrints/BP_EnemyAdvanced.BP_EnemyAdvanced_C") 0 (Transformation|GetWorldLocation (Variables|Default|GetSpawnPoint2)) "0, 0, 0" false 0)
      (AI|SpawnAIFromClass (Utilities|Select :Index (Math|Random|RandomInteger 3) :Option%200 "/Game/Tyler/Bluebrints/BP_EnemyBasic.BP_EnemyBasic_C" :Option%201 "/Game/Tyler/Bluebrints/BP_EnemyAdvanced.BP_EnemyAdvanced_C" :Option%202 "/Game/Tyler/Bluebrints/BP_EnemyAdvanced.BP_EnemyAdvanced_C" :Option%203 "/Game/Tyler/Bluebrints/BP_EnemyAdvanced.BP_EnemyAdvanced_C") 0 (Transformation|GetWorldLocation (Variables|Default|GetSpawnPoint1)) "0, 0, 0" false 0))))

(event Custom|SweepAttack
  (params (Player%20Target :type Actor%20Object%20Reference))
  ;[1 1 1] Sweep Attack
  (bind _asbp_third_person_character_synty (Utilities|Casting|CastToBP_ThirdPersonCharacterSynty Player%20Target))
  (Default|TakeDamage _asbp_third_person_character_synty 2e+01))

(event Custom|RandomAttack
  (params (Target%20Player :type Actor%20Object%20Reference))
  ;[1 1 1] Pick A random attack
  (Development|PrintString "randAttack")
  (switch int (Math|Random|RandomInteger 5)
    (:Default
      (CallFunction|SharkAttack Target%20Player :!label _label))
    (:0
      (goto _label))
    (:1
      (goto _label))
    (:2
      (CallFunction|SpawnMoreSkels Target%20Player :!label _label_2))
    (:3
      (goto _label_2))
    (:4
      (goto _label))
    (:5
      (goto _label)))
  (Utilities|FlowControl|Delay (Math|Random|RandomFloatinRange 3.0 1e+01))
  (CallFunction|RandomAttack Target%20Player))

(event Custom|AddStagger
  (bind _charactermovement (Variables|Character|GetCharacterMovement))
  ;[1 1 1] Stagger enemy
  (Variables|/Script/Engine.CharacterMovementComponent|SetMaxWalkSpeed _charactermovement 0.0)
  (Utilities|FlowControl|Delay 0.2)
  (Variables|/Script/Engine.CharacterMovementComponent|SetMaxWalkSpeed _charactermovement 2e+02))

(event EventBeginPlay
  (bind _self self)
  (bind _capsulecomponent (Variables|Collision|GetCapsuleComponent _self))
  (bind _returnvalue (Transformation|GetWorldLocation _capsulecomponent))
  ;[1 1 1] Enemy Move
  (CallFunction|UpdateHealthWidget)
  ;;[1 1 1] Ref to sky timer
  (bind _outactors (Actor|GetAllActorsOfClass "/Game/Tyler/Bluebrints/Bp_SkyTimer.Bp_SkyTimer_C"))
  (Variables|Default|SetSkyTimerRef (Utilities|Array|Get(acopy) _outactors))
  (bind _outactors_2 (Actor|GetAllActorsOfClass "/Game/ThirdPerson/Blueprints/BP_ThirdPersonCharacterSynty.BP_ThirdPersonCharacterSynty_C"))
  (CallFunction|RandomAttack (select (> (Math|Vector|Distance(Vector) (Math|Vector|MakeVector (.x _returnvalue) (.y _returnvalue) 0.0) (Math|Vector|MakeVector (.x (Transformation|GetWorldLocation (Variables|/Script/Engine.Character|GetCapsuleComponent (Utilities|Array|Get(acopy) _outactors_2)))) (.y (Transformation|GetWorldLocation (Variables|/Script/Engine.Character|GetCapsuleComponent (Utilities|Array|Get(acopy) _outactors_2)))) 0.0)) (Math|Vector|Distance(Vector) (Math|Vector|MakeVector (.x _returnvalue) (.y _returnvalue) 0.0) (Math|Vector|MakeVector (.x (Transformation|GetWorldLocation (Variables|/Script/Engine.Character|GetCapsuleComponent (Utilities|Array|Get(acopy) _outactors_2 1)))) (.y (Transformation|GetWorldLocation (Variables|/Script/Engine.Character|GetCapsuleComponent (Utilities|Array|Get(acopy) _outactors_2 1)))) 0.0))) (Utilities|Array|Get(acopy) _outactors_2 1) (Utilities|Array|Get(acopy) _outactors_2)))
  (AI|AIMoveTo self "0, 0, 0" (select (> (Math|Vector|Distance(Vector) (Math|Vector|MakeVector (.x _returnvalue) (.y _returnvalue) 0.0) (Math|Vector|MakeVector (.x (Transformation|GetWorldLocation (Variables|/Script/Engine.Character|GetCapsuleComponent (Utilities|Array|Get(acopy) _outactors_2)))) (.y (Transformation|GetWorldLocation (Variables|/Script/Engine.Character|GetCapsuleComponent (Utilities|Array|Get(acopy) _outactors_2)))) 0.0)) (Math|Vector|Distance(Vector) (Math|Vector|MakeVector (.x _returnvalue) (.y _returnvalue) 0.0) (Math|Vector|MakeVector (.x (Transformation|GetWorldLocation (Variables|/Script/Engine.Character|GetCapsuleComponent (Utilities|Array|Get(acopy) _outactors_2 1)))) (.y (Transformation|GetWorldLocation (Variables|/Script/Engine.Character|GetCapsuleComponent (Utilities|Array|Get(acopy) _outactors_2 1)))) 0.0))) (Utilities|Array|Get(acopy) _outactors_2 1) (Utilities|Array|Get(acopy) _outactors_2)) 5.0 false :!label _label
    (:then
      _)
    (:OnSuccess
      (Utilities|FlowControl|DoOnce false :!label _label_2
        (:Completed
          (if (> (Math|Vector|Distance(Vector) (Math|Vector|MakeVector (.x _returnvalue) (.y _returnvalue) 0.0) (Math|Vector|MakeVector (.x (Transformation|GetWorldLocation (Variables|/Script/Engine.Character|GetCapsuleComponent (Utilities|Array|Get(acopy) _outactors_2)))) (.y (Transformation|GetWorldLocation (Variables|/Script/Engine.Character|GetCapsuleComponent (Utilities|Array|Get(acopy) _outactors_2)))) 0.0)) (Math|Vector|Distance(Vector) (Math|Vector|MakeVector (.x _returnvalue) (.y _returnvalue) 0.0) (Math|Vector|MakeVector (.x (Transformation|GetWorldLocation (Variables|/Script/Engine.Character|GetCapsuleComponent (Utilities|Array|Get(acopy) _outactors_2 1)))) (.y (Transformation|GetWorldLocation (Variables|/Script/Engine.Character|GetCapsuleComponent (Utilities|Array|Get(acopy) _outactors_2 1)))) 0.0))) ; Player 2 true, player 1 false
            ;;[1 1 1] Damage
            (CallFunction|SweepAttack (Utilities|Array|Get(acopy) _outactors_2 1)) ; Player2
            (else
              (CallFunction|SweepAttack (Utilities|Array|Get(acopy) _outactors_2)) ; Player1
            ))
          (Animation|PlayAnimMontage "/Game/Developers/dynod/SwingBoss.SwingBoss" 1.0 "None")
          (Utilities|FlowControl|Delay 1.0)
          (goto _label_2 Reset))))
    (:OnFail
      _))
  (Utilities|FlowControl|Delay 1.0)
  (Animation|PlayAnimMontage "/Game/Developers/dynod/SmallAttack.SmallAttack" 1.0 "None")
  (goto _label))

(event EventTick
  (params (DeltaSeconds :type Float%20%28single-precision%29))
  ;[1 1 1] Check if day
)

(fn ConstructionScript)