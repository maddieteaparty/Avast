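; Sword pickup that attaches to the Synty third-person character's weapon socket and has two upgrade stages.
; Capsule overlap with that character disables collision on the wooden and short sword meshes, then snaps the weapon to the socket.
; SwordUpgrade first swaps wooden for short sword, then reveals NSwordUpgrade, raising SwordDamage each time.
; BeginPlay fires both upgrades on timed delays, independent of pickup.
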(event OnComponentBeginOverlap(Capsule)
  (params (OverlappedComponent :type Primitive%20Component%20Object%20Reference) (OtherActor :type Actor%20Object%20Reference) (OtherComp :type Primitive%20Component%20Object%20Reference) (OtherBodyIndex :type Integer) (bFromSweep :type Boolean) (SweepResult :type Hit%20Result%20Structure%20%28by%20ref%29))
  ;[1 1 1] Sword Pick up
  (bind _asbp_third_person_character_synty (Utilities|Casting|CastToBP_ThirdPersonCharacterSynty OtherActor))
  (Collision|SetCollisionEnabled (Variables|Default|GetSM_Wep_Wooden_01) "NoCollision")
  (Transformation|AttachComponentToComponent (Variables|/Game/ThirdPerson/Blueprints/BP_ThirdPersonCharacterSynty.BP_ThirdPersonCharacterSynty_C|GetWeaponSocket _asbp_third_person_character_synty) "None" "SnapToTarget" "SnapToTarget" "SnapToTarget" true))

(event Custom|SwordUpgrade
  ;[1 1 1] Both sword upgrades
  (if (Variables|Default|GetFirstUpgrade)
    (Rendering|SetVisibility (Variables|Default|GetSM_Wep_Wooden_01) false false)
    (Rendering|SetVisibility (Variables|Default|GetSM_Wep_Shortsword_02) true false)
    (Variables|Default|SetSwordDamage 5e+01)
    (Variables|Default|SetFirstUpgrade false)
    (else
      (Rendering|SetVisibility (Variables|Default|GetN_SwordUpgrade) true false)
      (Variables|Default|SetSwordDamage 1e+02))))

(event EventBeginPlay
  (Utilities|FlowControl|Delay 1e+01)
  (CallFunction|SwordUpgrade)
  (Utilities|FlowControl|Delay 5.0)
  (CallFunction|SwordUpgrade))

(event Collision|EventActorBeginOverlap
  (params (OtherActor :type Actor%20Object%20Reference)))

(event EventTick
  (params (DeltaSeconds :type Float%20%28single-precision%29)))

(fn ConstructionScript)