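; BP_SpawnerForBoss is a spawn point, named for a boss encounter, that creates one AI enemy at its root location whenever SpawnSkels is called.
; A random switch picks either BP_EnemyBasic or a coin flip between it and BP_EnemyAdvanced.
; The third, advanced-weighted branch is unreachable because RandomInteger(2) returns only 0 or 1.
; Despite the "based on night" comment, the choice reads no night state.
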(event Custom|SpawnSkels
  ;[1 1 1] spawn enemy based on night
  (switch int (Math|Random|RandomInteger 2)
    (:Default
      (AI|SpawnAIFromClass "/Game/Tyler/Bluebrints/BP_EnemyBasic.BP_EnemyBasic_C" 0 (Transformation|GetWorldLocation (Variables|Default|GetDefaultSceneRoot self)) "0, 0, 0" false 0 :!label _label))
    (:0
      (goto _label))
    (:1
      (AI|SpawnAIFromClass (select (Math|Random|RandomBool) "/Game/Tyler/Bluebrints/BP_EnemyAdvanced.BP_EnemyAdvanced_C" "/Game/Tyler/Bluebrints/BP_EnemyBasic.BP_EnemyBasic_C") 0 (Transformation|GetWorldLocation (Variables|Default|GetDefaultSceneRoot self)) "0, 0, 0" false 0))
    (:2
      (AI|SpawnAIFromClass (Utilities|Select :Index (Math|Random|RandomInteger 3) :Option%200 "/Game/Tyler/Bluebrints/BP_EnemyBasic.BP_EnemyBasic_C" :Option%201 "/Game/Tyler/Bluebrints/BP_EnemyAdvanced.BP_EnemyAdvanced_C" :Option%202 "/Game/Tyler/Bluebrints/BP_EnemyAdvanced.BP_EnemyAdvanced_C" :Option%203 "/Game/Tyler/Bluebrints/BP_EnemyAdvanced.BP_EnemyAdvanced_C") 0 (Transformation|GetWorldLocation (Variables|Default|GetDefaultSceneRoot self)) "0, 0, 0" false 0))))

(event Collision|EventActorBeginOverlap
  (params (OtherActor :type Actor%20Object%20Reference)))

(fn ConstructionScript)