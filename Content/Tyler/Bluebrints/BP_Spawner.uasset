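; BP_Spawner is a placed enemy spawner that spawns AI pawns at its own location during the night.
; On BeginPlay it caches the Bp_SkyTimer; a Delay on Tick throttles spawn attempts to random intervals, each gated by the timer's night flag.
; The night number selects a difficulty tier, shifting spawns from only BP_EnemyBasic to random mixes increasingly weighted toward BP_EnemyAdvanced.
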(event EventBeginPlay
  ;[1 1 1] Ref to sky timer
  (bind _outactors (Actor|GetAllActorsOfClass "/Game/Tyler/Bluebrints/Bp_SkyTimer.Bp_SkyTimer_C"))
  (Variables|Default|SetRef%20to%20timer (Utilities|Array|Get(acopy) _outactors)))

(event Collision|EventActorBeginOverlap
  (params (OtherActor :type Actor%20Object%20Reference)))

(event EventTick
  (params (DeltaSeconds :type Float%20%28single-precision%29))
  (bind _ref_to_timer (Variables|Default|GetRef%20to%20timer))
  ;[1 1 1] spawn enemy based on night
  (Utilities|FlowControl|Delay (Math|Random|RandomFloatinRange 5.0 2e+01))
  (if (Variables|/Game/Tyler/Bluebrints/Bp_SkyTimer.Bp_SkyTimer_C|GetNightTimer _ref_to_timer) ; checks if it is night
    (Variables|Default|SetNightDif (Utilities|Select :Index (Variables|/Game/Tyler/Bluebrints/Bp_SkyTimer.Bp_SkyTimer_C|GetNightNumber _ref_to_timer) :Option%200 0 :Option%201 0 :Option%202 1 :Option%203 1 :Option%204 2 :Option%205 2))
    (switch int (Variables|Default|GetNightDif)
      (:Default
        (AI|SpawnAIFromClass "/Game/Tyler/Bluebrints/BP_EnemyBasic.BP_EnemyBasic_C" 0 (Transformation|GetWorldLocation (Variables|Default|GetDefaultSceneRoot self)) "0, 0, 0" false 0 :!label _label))
      (:0
        (goto _label))
      (:1
        (AI|SpawnAIFromClass (select (Math|Random|RandomBool) "/Game/Tyler/Bluebrints/BP_EnemyAdvanced.BP_EnemyAdvanced_C" "/Game/Tyler/Bluebrints/BP_EnemyBasic.BP_EnemyBasic_C") 0 (Transformation|GetWorldLocation (Variables|Default|GetDefaultSceneRoot self)) "0, 0, 0" false 0))
      (:2
        (AI|SpawnAIFromClass (Utilities|Select :Index (Math|Random|RandomInteger 3) :Option%200 "/Game/Tyler/Bluebrints/BP_EnemyBasic.BP_EnemyBasic_C" :Option%201 "/Game/Tyler/Bluebrints/BP_EnemyAdvanced.BP_EnemyAdvanced_C" :Option%202 "/Game/Tyler/Bluebrints/BP_EnemyAdvanced.BP_EnemyAdvanced_C" :Option%203 "/Game/Tyler/Bluebrints/BP_EnemyAdvanced.BP_EnemyAdvanced_C") 0 (Transformation|GetWorldLocation (Variables|Default|GetDefaultSceneRoot self)) "0, 0, 0" false 0)))))

(fn ConstructionScript)